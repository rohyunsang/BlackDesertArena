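; Battle royale shrinking safe zone actor that notifies actors entering or leaving its mesh via server-side overlap messages and can spawn a zone widget.
; The server advances ZoneSteps through hold and move phases, choosing a random offset center and updating a countdown every second.
; StartMovingZone moves the zone on all clients, using a looping timer to lerp mesh scale and location.
; Radii step linearly from start toward end, normalized by mesh bounds.
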(event OnComponentEndOverlap(ZoneMesh)
  (params (OverlappedComponent :type Primitive%20Component%20Object%20Reference) (OtherActor :type Actor%20Object%20Reference) (OtherComp :type Primitive%20Component%20Object%20Reference) (OtherBodyIndex :type Integer))
  ;[1 1 1] Damage actor if he no in zone
  (Networking|SwitchHasAuthority
    (:Authority
      (Class|BIBRInterface|NotinZone(Message) OtherActor 2.0))))

(event OnComponentBeginOverlap(ZoneMesh)
  (params (OverlappedComponent :type Primitive%20Component%20Object%20Reference) (OtherActor :type Actor%20Object%20Reference) (OtherComp :type Primitive%20Component%20Object%20Reference) (OtherBodyIndex :type Integer) (bFromSweep :type Boolean) (SweepResult :type Hit%20Result%20Structure%20%28by%20ref%29))
  ;[1 1 1] Stop damage actor if he in zone
  (Networking|SwitchHasAuthority
    (:Authority
      (Class|BIBRInterface|InZone(Message) OtherActor))))

(event Custom|StartMovingZone
  (params (CurrentStepRadius :type Float%20%28single-precision%29) (NextStepRadius :type Float%20%28single-precision%29) (CurrentStepLocation :type Vector) (NextStepLocation :type Vector) (MovingTime :type Float%20%28single-precision%29))
  ;[1 1 1] Move zone on all clients
  (CallFunction|MoveZone CurrentStepRadius NextStepRadius CurrentStepLocation NextStepLocation MovingTime))

(event EventBeginPlay
  ;[1 1 1] Initialize zone
  (CallFunction|CreateZone)
  (if (Variables|Settings|GetCreateWidget) ; Create widget if needed
    (bind _returnvalue (UserInterface|CreateWidget "/Game/BatteRoyaleZone/Blueprints/BP_BRZoneWidget.BP_BRZoneWidget_C"))
    (UserInterface|Viewport|AddtoViewport _returnvalue 0)))

(event EventTick
  (params (DeltaSeconds :type Float%20%28single-precision%29))
  (CallFunction|TickTimer DeltaSeconds) ; Current zone step timer
)

(fn ConstructionScript
  (bind _zonemesh (Variables|Default|GetZoneMesh))
  ;[1 1 1] Get mesh radius and set zone size
  (Transformation|SetWorldScale3D _zonemesh "1.000000,1.000000,1.000000")
  (Variables|Debug|SetMeshRadius (.x (.BoxExtent (Collision|GetComponentBounds _zonemesh))))
  (Transformation|SetWorldScale3D _zonemesh (Math|Vector|MakeVector (/ (Variables|Settings|GetStartRadius) (Variables|Debug|GetMeshRadius)) (/ (Variables|Settings|GetStartRadius) (Variables|Debug|GetMeshRadius)) (/ (Variables|Settings|GetZoneHeight) (Variables|Debug|GetMeshRadius)))))

(fn CreateZone
  (Networking|SwitchHasAuthority ; Only on server
    (:Authority
      (CallFunction|NewStep) ; Initialize first step
      (Utilities|Time|SetTimerbyFunctionName 0 "SendTimeToPlayers" 1.0 true) ; Send time to players
    )))

(fn TickTimer
  (params (Delta :type Float%20%28single-precision%29))
  (bind (_currentstepradius _nextstepradius) (CallFunction|GetRadius))
  (bind _zonesteps (Variables|Settings|GetZoneSteps))
  (bind _currentstep (Variables|Debug|GetCurrentStep))
  (bind _zonemesh (Variables|Default|GetZoneMesh))
  (bind _nextstepradius_2 (Variables|Debug|GetNextStepRadius))
  (bind _currentstepradius_2 (Variables|Debug|GetCurrentStepRadius))
  (bind _returnvalue (- _currentstepradius_2 _nextstepradius_2))
  (bind _returnvalue_2 (Transformation|GetWorldLocation _zonemesh))
  (bind _output (Utilities|Array|Get(acopy) _zonesteps _currentstep))
  (bind (_holdtime _movingtime) (Utilities|Struct|BreakBP_ZoneStruct _output))
  (bind _returnvalue_3 (* _returnvalue -1.0))
  (Networking|SwitchHasAuthority ; Only on server
    (:Authority
      ;[1 1 1] Increase current step timer
      (Variables|Debug|SetTimeAfterStartStep (+ Delta (Variables|Debug|GetTimeAfterStartStep)))
      (if (not (< (Variables|Debug|GetTimeAfterStartStep) _holdtime)) ; Timer less than hold time
        (if (< (Variables|Debug|GetTimeAfterStartStep) (+ _holdtime _movingtime)) ; Timer less than moving time
          (if (not (Variables|Debug|GetMoving?)) ; Start moving
            (Variables|Debug|SetMoving? true)
            (CallFunction|StartMovingZone _currentstepradius _nextstepradius _returnvalue_2 (+ _returnvalue_2 (Math|Vector|MakeVector (* (Math|Random|RandomFloatinRange _returnvalue_3 _returnvalue) 0.7) (* (Math|Random|RandomFloatinRange _returnvalue_3 _returnvalue) 0.7) 0.0)) _movingtime))
          (else
            ;[1 1 1] Initialize new step if moving done
            (CallFunction|NewStep)
            (Variables|Debug|SetMoving? false)))))))

(fn NewStep
  ;[1 1 1] Reset timer and increase current step
  (if (> (+ (Variables|Debug|GetCurrentStep) 1) (Utilities|Array|LastIndex (Variables|Settings|GetZoneSteps)))
    (Utilities|Time|ClearTimerbyFunctionName 0 "SendTimeToPlayers")
    (Variables|Debug|SetLastStep true)
    (else
      (Variables|Debug|SetTimeAfterStartStep 0.0)
      (Variables|Debug|SetCurrentStep (+ (Variables|Debug|GetCurrentStep) 1)))))

(fn GetRadius
  (bind _currentstep (Variables|Debug|GetCurrentStep))
  (bind _zonesteps (Variables|Settings|GetZoneSteps))
  (bind _endradius (Variables|Settings|GetEndRadius))
  (bind _startradius (Variables|Settings|GetStartRadius))
  (bind _returnvalue (Utilities|Array|Length _zonesteps))
  (bind _returnvalue_2 (- _startradius _endradius))
  (bind _returnvalue_3 (Math|Conversions|ToFloat(Integer) _currentstep))
  (bind _returnvalue_4 (+ _returnvalue 0))
  (bind _returnvalue_5 (Math|Conversions|ToFloat(Integer) _returnvalue_4))
  (bind _returnvalue_6 (/ _returnvalue_2 _returnvalue_5))
  (return (- (Variables|Settings|GetStartRadius) (* _returnvalue_6 _returnvalue_3)) (- (Variables|Settings|GetStartRadius) (* _returnvalue_6 (+ _returnvalue_3 1.0)))))

(fn MoveZoneTick
  (bind _zonemesh (Variables|Default|GetZoneMesh))
  ;[1 1 1] Increase alpha
  (Variables|Debug|SetMovingAlpha (Math|Float|Clamp(Float) (+ (Variables|Debug|GetMovingAlpha) (Variables|Debug|GetMovingAlphaDelta))))
  ;[1 1 1] Calculate and set radius and location
  (Transformation|SetWorldScale3D _zonemesh (Math|Vector|MakeVector (/ (Math|Float|Lerp (Variables|Debug|GetCurrentStepRadius) (Variables|Debug|GetNextStepRadius) (Variables|Debug|GetMovingAlpha)) (Variables|Debug|GetMeshRadius)) (/ (Math|Float|Lerp (Variables|Debug|GetCurrentStepRadius) (Variables|Debug|GetNextStepRadius) (Variables|Debug|GetMovingAlpha)) (Variables|Debug|GetMeshRadius)) (/ (Variables|Settings|GetZoneHeight) (Variables|Debug|GetMeshRadius))))
  (Transformation|SetWorldLocation _zonemesh (Math|Vector|Lerp(Vector) (Variables|Debug|GetCurrentStepLocation) (Variables|Debug|GetNextStepLocation) (Variables|Debug|GetMovingAlpha)) false false)
  ;[1 1 1] Stop moving if alpha >= 1
  (if (>= (Variables|Debug|GetMovingAlpha) 1.0)
    (Utilities|Time|ClearTimerbyFunctionName 0 "MoveZoneTick")))

(fn MoveZone
  (params (CurrentStepRadius :type Float%20%28single-precision%29) (NextStepRadius :type Float%20%28single-precision%29) (CurrentStepLocation :type Vector) (NextStepLocation :type Vector) (MovingTime :type Float%20%28single-precision%29))
  ;[1 1 1] Initialize radius and location
  (Variables|Debug|SetCurrentStepRadius CurrentStepRadius)
  (Variables|Debug|SetNextStepRadius NextStepRadius)
  (Variables|Debug|SetCurrentStepLocation CurrentStepLocation)
  (Variables|Debug|SetNextStepLocation NextStepLocation)
  (Variables|Debug|SetMovingAlpha 0.0)
  (Variables|Debug|SetMovingAlphaDelta (/ 0.01 MovingTime))
  (Utilities|Time|SetTimerbyFunctionName 0 "MoveZoneTick" 0.01 true) ; Move
)

(fn GetTimeto
  (bind _timeafterstartstep (Variables|Debug|GetTimeAfterStartStep))
  (bind _zonesteps (Variables|Settings|GetZoneSteps))
  (bind _currentstep (Variables|Debug|GetCurrentStep))
  (bind _output (Utilities|Array|Get(acopy) _zonesteps _currentstep))
  (bind (_holdtime _movingtime) (Utilities|Struct|BreakBP_ZoneStruct _output))
  (return (select (> _timeafterstartstep _holdtime) (- (+ _holdtime _movingtime) _timeafterstartstep) (- _holdtime _timeafterstartstep))))

(fn SendTimetoPlayers
  ;[1 1 1] Send time to all players
  (Variables|Debug|SetTime (CallFunction|GetTimeto)))